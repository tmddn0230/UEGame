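; Tower actor that builds a closed circular spline path in its local space when play begins.
; GeneratePath clears the spline, places evenly spaced points using cosine and sine from a point count and radius, then closes the loop and flags the path valid.
; Logic to move the Tower component along the spline with looping exists but is disconnected, so the tower does not move.
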(event EventBeginPlay
  (CallFunction|GeneratePath))

(event Collision|EventActorBeginOverlap
  (params (OtherActor :type Actor%20Object%20Reference)))

(event EventTick
  (params (DeltaSeconds :type Float%20%28single-precision%29)))

(fn ConstructionScript)

(fn GeneratePath
  (bind _radios (Variables|Default|GetRadios))
  ;[0.15 0.15 0.15 0.5] 1. 기본 포인트 삭제
  (Spline|ClearSplinePoints (Variables|Default|GetSpline) true)
  ;[0.15 0.15 0.15 0.5] 2. 원기둥의 중점을 가져온다.
  (LocalVariables|SetCilinderLoc (Variables|/Script/Engine.SceneComponent|GetRelativeLocation (Variables|Default|GetTower)))
  (for _index (range 0 (- (Variables|Default|GetNumDots) 1))
    ;[0.15 0.15 0.15 0.5] 8. Point 추가
    (Spline|AddSplinePoint (Variables|Default|GetSpline) (Math|Vector|MakeVector (* (Math|Trig|Cos(Radians) (* (/ (* 2.0 (Math|Trig|GetPI)) (Variables|Default|GetNumDots)) _index)) _radios) (* _radios (Math|Trig|Sin(Radians) (* (/ (* 2.0 (Math|Trig|GetPI)) (Variables|Default|GetNumDots)) _index))) 0.0) "Local" false))
  ;[0.15 0.15 0.15 0.5] 9. 루프 잠금
  (Spline|SetClosedLoop (Variables|Default|GetSpline) true true)
  (Variables|Default|SetIsValidPath? true))