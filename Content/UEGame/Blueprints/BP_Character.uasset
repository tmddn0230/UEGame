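; Character that moves along the spline of the level's BP_Tower and aims with the mouse while firing.
; When not firing, Tick turns AxisValue into spline speed and, if ready, places the actor at fixed height, facing travel or sideways when idle.
; Distance wraps at the spline ends when looping is on.
; While firing, movement stops updating and SpineRot follows the deprojected cursor ray's direction; otherwise it resets to zero.
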(event EventBeginPlay
  (bind _returnvalue (Actor|GetActorOfClass "/Game/UEGame/Blueprints/BP_Tower.BP_Tower_C"))
  (bind _output_get (Variables|Default|SetTower _returnvalue))
  (Variables|Default|SetSpline (Variables|/Game/UEGame/Blueprints/BP_Tower.BP_Tower_C|GetSpline _output_get)))

(event Collision|EventActorBeginOverlap
  (params (OtherActor :type Actor%20Object%20Reference)))

(event EventTick
  (params (DeltaSeconds :type Float%20%28single-precision%29))
  (bind _returnvalue (Game|GetPlayerController 0))
  (bind _spline (Variables|Default|GetSpline))
  (bind _axisvalue (Variables|Default|GetAxisValue))
  (bind _axisvalue_2 (Variables|Default|GetAxisValue))
  (bind _returnvalue_2 (Spline|GetSplineLength _spline))
  (bind (_locationx _locationy) (Game|Player|GetMousePosition _returnvalue))
  (bind (_worldposition _worlddirection) (Class|GameplayStatics|DeprojectScreentoWorld _returnvalue (Math|Vector2D|MakeVector2D _locationx _locationy)))
  (if (not (Variables|Default|GetIsFire))
    (Variables|Default|SetSpineRot "0, 0, 0")
    (Utilities|FlowControl|Sequence
      (:then_0
        (if (== _axisvalue 0.0)
          (Variables|Default|SetSplineSpeed 0.0)
          (else
            (Variables|Default|SetSplineSpeed (* _axisvalue -5e+02)))))
      (:then_1
        (if (Variables|Default|GetIsReady?)
          (Variables|Default|SetDistance%20Along%20Spline (+ (* DeltaSeconds (Variables|Default|GetSplineSpeed)) (Variables|Default|GetDistance%20Along%20Spline)))
          (Transformation|SetActorLocation (Math|Vector|MakeVector (.x (.location (Spline|GetTransformatDistanceAlongSpline (Variables|Default|GetSpline) (Variables|Default|GetDistance%20Along%20Spline) "World" false))) (.y (.location (Spline|GetTransformatDistanceAlongSpline (Variables|Default|GetSpline) (Variables|Default|GetDistance%20Along%20Spline) "World" false))) 89.0) false false)
          (if (== _axisvalue_2 0.0)
            (Transformation|SetActorRotation (Math|Rotator|MakeRotator (.roll (.rotation (Spline|GetTransformatDistanceAlongSpline (Variables|Default|GetSpline) (Variables|Default|GetDistance%20Along%20Spline) "World" false))) (.pitch (.rotation (Spline|GetTransformatDistanceAlongSpline (Variables|Default|GetSpline) (Variables|Default|GetDistance%20Along%20Spline) "World" false))) (+ (.yaw (.rotation (Spline|GetTransformatDistanceAlongSpline (Variables|Default|GetSpline) (Variables|Default|GetDistance%20Along%20Spline) "World" false))) 9e+01)))
            (elif (== _axisvalue_2 -1.0)
              (Transformation|SetActorRotation (Math|Rotator|MakeRotator (.roll (.rotation (Spline|GetTransformatDistanceAlongSpline (Variables|Default|GetSpline) (Variables|Default|GetDistance%20Along%20Spline) "World" false))) (.pitch (.rotation (Spline|GetTransformatDistanceAlongSpline (Variables|Default|GetSpline) (Variables|Default|GetDistance%20Along%20Spline) "World" false))) (.yaw (.rotation (Spline|GetTransformatDistanceAlongSpline (Variables|Default|GetSpline) (Variables|Default|GetDistance%20Along%20Spline) "World" false)))))
              (else
                (Transformation|SetActorRotation (Math|Rotator|MakeRotator (.roll (.rotation (Spline|GetTransformatDistanceAlongSpline (Variables|Default|GetSpline) (Variables|Default|GetDistance%20Along%20Spline) "World" false))) (.pitch (.rotation (Spline|GetTransformatDistanceAlongSpline (Variables|Default|GetSpline) (Variables|Default|GetDistance%20Along%20Spline) "World" false))) (+ (.yaw (.rotation (Spline|GetTransformatDistanceAlongSpline (Variables|Default|GetSpline) (Variables|Default|GetDistance%20Along%20Spline) "World" false))) 1.8e+02))))))
          (if (Variables|Default|GetIsLoop?)
            (if (> (Variables|Default|GetDistance%20Along%20Spline) _returnvalue_2)
              (Variables|Default|SetDistance%20Along%20Spline 0.0)
              (elif (< (Variables|Default|GetDistance%20Along%20Spline) 0.0)
                (Variables|Default|SetDistance%20Along%20Spline _returnvalue_2)))))))
    (else
      (bind _outhit (Collision|LineTraceByChannel _worldposition (+ _worldposition (* _worlddirection "10000.000000,10000.000000,10000.000000")) "TraceTypeQuery1" false 0 "None"))
      (Variables|Default|SetSpineRot (Math|Rotator|MakeRotator (.roll (Math|Rotator|FindLookatRotation (.tracestart _outhit) (.traceend _outhit))) (.pitch (Math|Rotator|FindLookatRotation (.tracestart _outhit) (.traceend _outhit))) (+ (.yaw (Math|Rotator|FindLookatRotation (.tracestart _outhit) (.traceend _outhit))) 1.8e+02))))))

(fn ConstructionScript)